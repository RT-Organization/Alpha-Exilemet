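; Night light actor for Forest of Spikes that drives a wandering, flickering point light.
; A looping Timeline at half play rate lerps the light to random horizontal points within MovementRange of the actor, picking a new target whenever it finishes.
; In parallel, a self-calling Flick event randomizes intensity up to NewIntensity after short random delays.
; The construction script applies the configured intensity and attenuation radius.
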(event Custom|PlayNow
  (bind _movement_range (Variables|Default|GetMovement%20range))
  (bind _returnvalue (* _movement_range -1.0))
  ;[0.15 0.15 0.15 0.5] Light movement target location
  (Variables|Default|SetNext%20location (+ (Transformation|GetActorLocation) (Math|Vector|MakeVector (Math|Random|RandomFloatinRange _returnvalue (Variables|Default|GetMovement%20range)) (Math|Random|RandomFloatinRange _returnvalue (Variables|Default|GetMovement%20range)) 0.0)))
  ;[0.15 0.15 0.15 0.5] Update alpha for locations
  (bind _alpha (Timeline|Timeline PlayFromStart)
    (:Update
      ;[0.15 0.15 0.15 0.5] Move light
      (Transformation|SetWorldLocation (Variables|Default|GetPointLight) (Math|Vector|Lerp(Vector) (Variables|Default|GetCurrent%20location) (Variables|Default|GetNext%20location) _alpha) false false))
    (:Finished
      ;[0.15 0.15 0.15 0.5] Current location as start location.
      (Variables|Default|SetCurrent%20location (Transformation|GetWorldLocation (Variables|Default|GetPointLight)))
      (CallFunction|PlayNow))))

(event Custom|Flick
  ;[0.15 0.15 0.15 0.5] Random delay
  (Utilities|FlowControl|Delay (Math|Random|RandomFloatinRange 0.02 0.1))
  ;[0.15 0.15 0.15 0.5] Set light intensity and start again
  (Rendering|Components|Light|SetIntensity (Variables|Default|GetPointLight) (Math|Random|RandomFloatinRange 0.0 (Variables|Default|GetNew%20Intensity)))
  (CallFunction|Flick))

(event EventBeginPlay
  (bind _movement_range (Variables|Default|GetMovement%20range))
  (bind _returnvalue (* _movement_range -1.0))
  ;[0.15 0.15 0.15 0.5] Start location to variable
  (Variables|Default|SetCurrent%20location (Transformation|GetActorLocation))
  ;[0.15 0.15 0.15 0.5] Timeline playback rate
  (Components|Timeline|SetPlayRate (Variables|Default|GetTimeline) 0.5)
  ;[0.15 0.15 0.15 0.5] 1st start movement then flickering
  (Utilities|FlowControl|Sequence
    (:then_0
      ;[0.15 0.15 0.15 0.5] Light movement target location
      (Variables|Default|SetNext%20location (+ (Transformation|GetActorLocation) (Math|Vector|MakeVector (Math|Random|RandomFloatinRange _returnvalue (Variables|Default|GetMovement%20range)) (Math|Random|RandomFloatinRange _returnvalue (Variables|Default|GetMovement%20range)) 0.0)))
      ;[0.15 0.15 0.15 0.5] Update alpha for locations
      (bind _alpha (Timeline|Timeline PlayFromStart)
        (:Update
          ;[0.15 0.15 0.15 0.5] Move light
          (Transformation|SetWorldLocation (Variables|Default|GetPointLight) (Math|Vector|Lerp(Vector) (Variables|Default|GetCurrent%20location) (Variables|Default|GetNext%20location) _alpha) false false))
        (:Finished
          ;[0.15 0.15 0.15 0.5] Current location as start location.
          (Variables|Default|SetCurrent%20location (Transformation|GetWorldLocation (Variables|Default|GetPointLight)))
          (CallFunction|PlayNow))))
    (:then_1
      (CallFunction|Flick))))

(fn ConstructionScript
  ;[0.15 0.15 0.15 0.5] set default values
  (Rendering|Components|Light|SetIntensity (Variables|Default|GetPointLight) (Variables|Default|GetNew%20Intensity))
  (Rendering|Lighting|SetAttenuationRadius (Variables|Default|GetPointLight) (Variables|Default|GetNew%20Radius)))