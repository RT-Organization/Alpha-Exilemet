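; BP_Brain_Save handles saving and loading the third-person player's position and view through BP_Save_Load save slots.
; Savegame records the player transform and follow-camera transform into a new save object and writes it to the named slot.
; LoadGame teleports the player and restores control rotation, or calls save and load with empty slot names if the cast fails.
; A SaveEquip helper returns valid equipment's item struct, unused here.
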(event Custom|Save%20game
  (params (Slot%20save :type String))
  ;[1 1 1] Saving
  (Variables|Default|SetSlot%20save Slot%20save)
  (bind _returnvalue (SaveGame|CreateSaveGameObject "/Game/menuGameSystemPro/SaveLoad/BP_Save_Load.BP_Save_Load_C"))
  (bind _outputpin (|SaveLocationAndRotation _returnvalue))
  (SaveGame|SaveGametoSlot _outputpin (Variables|Default|GetSlot%20save)))

(event Custom|LoadGame
  (params (SlotName :type String))
  ;[1 1 1] Loading
  (bind _returnvalue (SaveGame|LoadGamefromSlot SlotName))
  (bind _asbp_save_load (Utilities|Casting|CastToBP_Save_Load _returnvalue)
    (:then
      (|LoadLocationAndRotation _asbp_save_load _asbp_save_load))
    (:CastFailed
      (CallFunction|SaveGame)
      (CallFunction|LoadGame))))

(event EventBeginPlay
  (bind _asbp_third_person_character (Utilities|Casting|CastToBP_ThirdPersonCharacter (Game|GetPlayerCharacter 0)))
  (Variables|Default|SetRef%20Player _asbp_third_person_character))

(fn ConstructionScript)