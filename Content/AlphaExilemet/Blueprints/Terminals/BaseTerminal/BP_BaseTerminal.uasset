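; Base terminal Blueprint that lets the player use an in-world terminal through an on-screen UI panel.
; When the terminal view is ready, it registers itself as the player's active terminal, hides the HUD, spawns the configurable widget class and switches to game-and-UI input with a cursor.
; Closing removes the widget, clears the player reference to the terminal, restores HUD and game-only input, then stops the interaction.
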(event Custom|CloseTerminal
  (bind _returnvalue (Game|GetPlayerController 0))
  (Widget|RemovefromParent (Variables|Default|GetActiveWidget))
  (Variables|/Game/AlphaExilemet/Blueprints/Character/BP_Player.BP_Player_C|SetActiveTerminal (Variables|Default|GetPlayerRef) 0)
  (Utilities|SetPlayerHUD "Visible")
  (Input|SetInputModeGameOnly _returnvalue false)
  (Variables|/Script/Engine.PlayerController|SetbShowMouseCursor _returnvalue false)
  (Class|BaseTerminal|StopTerminalInteraction (Variables|Default|GetPlayerRef)))

(event EventOnTerminalViewReady
  (params (Interactor :type Alpha%20Exilemet%20Character%20Object%20Reference))
  (bind _asbp_player (Utilities|Casting|CastToBP_Player Interactor))
  (Variables|Default|SetPlayerRef _asbp_player)
  (Variables|/Game/AlphaExilemet/Blueprints/Character/BP_Player.BP_Player_C|SetActiveTerminal _asbp_player self)
  (CallFunction|OpenTerminalPanel)
  (CallFunction|SetUiInput))

(fn ConstructionScript)

(fn SetUiInput
  (Input|SetInputModeGameandUI (Game|GetPlayerController 0) (Variables|Default|GetActiveWidget) "DoNotLock" false false)
  (Variables|/Script/Engine.PlayerController|SetbShowMouseCursor (Game|GetPlayerController 0) true))

(fn OpenTerminalPanel
  (bind _returnvalue (UserInterface|CreateWidget (Variables|Default|GetTerminalWidgetClass)))
  (bind _output_get (Variables|Default|SetActiveWidget _returnvalue))
  (Utilities|SetPlayerHUD "Hidden")
  (UserInterface|Viewport|AddtoViewport _output_get 0)
  (return))