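; Game instance for AlphaExilemet that loads or creates the player's audio and camera settings at startup.
; On Init it reads the "settings" save slot into CurrentSettings and applies the saved Master, Music and SFX volumes as sound class overrides on a sound mix.
; If that load or cast fails, it creates a new BP_SettingsSaveGame with default volumes and camera sensitivity, sets the overrides and saves to the slot.
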(event EventInit
  (bind _returnvalue (SaveGame|LoadGamefromSlot "settings"))
  (bind _asbp_settings_save_game (Utilities|Casting|CastToBP_SettingsSaveGame _returnvalue)
    (:then
      (Variables|Default|SetCurrentSettings _asbp_settings_save_game)
      ;[0.15 0.15 0.15 0.5] Load Settings Game
      (Audio|SetSoundMixClassOverride "/Game/menuGameSystemPro/Audios/Class/SCM_SoundClass_Mix.SCM_SoundClass_Mix" "/Game/menuGameSystemPro/Audios/Class/SC_Music.SC_Music" (Variables|/Game/menuGameSystemPro/SaveLoad/BP_SettingsSaveGame.BP_SettingsSaveGame_C|GetMusicVolume (Variables|Default|GetCurrentSettings)) 1.0 1.0 true)
      (Audio|SetSoundMixClassOverride "/Game/menuGameSystemPro/Audios/Class/SCM_SoundClass_Mix.SCM_SoundClass_Mix" "/Game/menuGameSystemPro/Audios/Class/SC_SFX.SC_SFX" (Variables|/Game/menuGameSystemPro/SaveLoad/BP_SettingsSaveGame.BP_SettingsSaveGame_C|GetSFXVolume (Variables|Default|GetCurrentSettings)) 1.0 1.0 true)
      (Audio|SetSoundMixClassOverride "/Game/menuGameSystemPro/Audios/Class/SCM_SoundClass_Mix.SCM_SoundClass_Mix" "/Game/menuGameSystemPro/Audios/Class/SC_SoundClass_Master.SC_SoundClass_Master" (Variables|/Game/menuGameSystemPro/SaveLoad/BP_SettingsSaveGame.BP_SettingsSaveGame_C|GetMasteVolume (Variables|Default|GetCurrentSettings)) 1.0 1.0 true))
    (:CastFailed
      (bind _returnvalue_2 (SaveGame|CreateSaveGameObject "/Game/menuGameSystemPro/SaveLoad/BP_SettingsSaveGame.BP_SettingsSaveGame_C"))
      (Variables|Default|SetCurrentSettings _returnvalue_2)
      ;[0.15 0.15 0.15 0.5] New Save Settings
      (bind _output_get (Variables|/Game/menuGameSystemPro/SaveLoad/BP_SettingsSaveGame.BP_SettingsSaveGame_C|SetMasteVolume (Variables|Default|GetCurrentSettings) 1.0))
      (Audio|SetSoundMixClassOverride "/Game/menuGameSystemPro/Audios/Class/SCM_SoundClass_Mix.SCM_SoundClass_Mix" "/Game/menuGameSystemPro/Audios/Class/SC_SoundClass_Master.SC_SoundClass_Master" _output_get 1.0 1.0 true)
      (bind _output_get_2 (Variables|/Game/menuGameSystemPro/SaveLoad/BP_SettingsSaveGame.BP_SettingsSaveGame_C|SetMusicVolume (Variables|Default|GetCurrentSettings) 1.0))
      (Audio|SetSoundMixClassOverride "/Game/menuGameSystemPro/Audios/Class/SCM_SoundClass_Mix.SCM_SoundClass_Mix" "/Game/menuGameSystemPro/Audios/Class/SC_Music.SC_Music" _output_get_2 1.0 1.0 true)
      (Variables|/Game/menuGameSystemPro/SaveLoad/BP_SettingsSaveGame.BP_SettingsSaveGame_C|SetSFXVolume (Variables|Default|GetCurrentSettings) 1.0)
      (Audio|SetSoundMixClassOverride "/Game/menuGameSystemPro/Audios/Class/SCM_SoundClass_Mix.SCM_SoundClass_Mix" "/Game/menuGameSystemPro/Audios/Class/SC_SFX.SC_SFX" 1.0 1.0 1.0 true)
      (Variables|/Game/menuGameSystemPro/SaveLoad/BP_SettingsSaveGame.BP_SettingsSaveGame_C|SetCameraSensitivityX (Variables|Default|GetCurrentSettings) 0.5)
      (Variables|/Game/menuGameSystemPro/SaveLoad/BP_SettingsSaveGame.BP_SettingsSaveGame_C|SetCameraSensitivityY (Variables|Default|GetCurrentSettings) 0.5)
      (SaveGame|SaveGametoSlot 0 "settings")
      (SaveGame|LoadGamefromSlot "settings"))))