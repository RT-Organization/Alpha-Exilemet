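; BP_MenuPlanet is the rotating main menu planet that performs the transition into a new game.
; StartNewGameTransition stops its RotatingMovement and uses a timeline to lerp the planet from its current rotation to a zero rotation along the shortest path.
; After a short delay it removes the main menu widget and asks the AlphaStreamingSubsystem to load the Tutorial level and unload MainMenu.
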(event Custom|StartNewGameTransition
  (params (MainMenuWidgetRef :type WB%20Main%20Menu%20Object%20Reference))
  (Variables|Default|SetMain%20Menu%20Widget%20Ref MainMenuWidgetRef)
  (Components|Activation|Deactivate (Variables|Default|GetRotatingMovement))
  (Variables|Default|SetStartRotation (Transformation|GetActorRotation))
  (bind _alpha (Timeline|AlignPlanet_TL Play)
    (:Update
      (Transformation|SetActorRotation (Math|Rotator|Lerp(Rotator) (Variables|Default|GetStartRotation) "0, 0, 0" _alpha true)))
    (:Finished
      (Utilities|FlowControl|Delay 0.5)
      (Widget|RemovefromParent (Variables|Default|GetMain%20Menu%20Widget%20Ref))
      (Class|AlphaStreamingSubsystem|StreamLevel (Subsystems|GetAlphaStreamingSubsystem) "Tutorial" "MainMenu"))))

(fn ConstructionScript)