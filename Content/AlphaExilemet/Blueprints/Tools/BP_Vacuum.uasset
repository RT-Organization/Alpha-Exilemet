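; BP_Vacuum is an equippable vacuum tool that plays lightning absorption effects when it hits a liquid.
; On a liquid hit, it looks up the resource's primary color in DT_Resources and spawns an attached Niagara lightning effect toward the liquid mesh, tinted with that color.
; Materializing drives a dissolve material parameter through a timeline, ignoring Visibility collision until it finishes.
; Equip and unequip defer to the parent class.
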(event EventOnLiquidHitting
  (params (Liquid :type Liquid%20Resource%20Object%20Reference))
  ;[0.15 0.15 0.15 0.5] VFX
  (bind _returnvalue (Utilities|GetDataTableRow "/Game/AlphaExilemet/Types/DT_Resources.DT_Resources" (.rowname (Variables|/Script/AlphaExilemet.ResourceBase|GetResourceID Liquid)))
    (:then
      (Utilities|MakeLightningAbsorbEffect (Transformation|GetWorldLocation (Variables|/Script/AlphaExilemet.LiquidResource|GetLiquidMesh Liquid)) (.primarycolor _returnvalue)))))

(event EventOnUnequip
  ;[0.15 0.15 0.15 0.5] Logic
  (|CallParentFunction))

(event EventOnEquip
  ;[0.15 0.15 0.15 0.5] Logic
  (|CallParentFunction))

(event EventMaterializeItem
  (Collision|SetCollisionResponsetoChannel (Variables|Character|GetMesh) "ECC_Visibility" "ECR_Ignore")
  (bind _alpha (Timeline|Timeline Play)
    (:Update
      (Rendering|Material|SetScalarParameterValueonMaterials (Variables|Character|GetMesh) "Disolve" _alpha))
    (:Finished
      (Collision|SetCollisionResponsetoChannel (Variables|Character|GetMesh) "ECC_Visibility" "ECR_Block"))))

(fn ConstructionScript)