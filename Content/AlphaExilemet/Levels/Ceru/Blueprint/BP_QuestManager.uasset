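; BP_QuestManager tracks an ordered pillar-symbol puzzle.
; PilastriAttivato compares each activated symbol to OrdineCorretto at PassoAttuale, advancing the step on a match and resetting it to zero on a mistake.
; Six correct activations in a row only print a solved message; the event graph holds just disabled default events, so calls must come from outside.
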(event EventBeginPlay)

(event Collision|EventActorBeginOverlap
  (params (OtherActor :type Actor%20Object%20Reference)))

(event EventTick
  (params (DeltaSeconds :type Float%20%28single-precision%29)))

(fn ConstructionScript)

(fn PilastriAttivato
  (params (SimboloAttivo :type Name))
  (Development|PrintString (Utilities|String|ToString(Integer) (Variables|Default|GetPassoAttuale)))
  (if (== (Utilities|Array|Get(acopy) (Variables|Default|GetOrdineCorretto) (Variables|Default|GetPassoAttuale)) SimboloAttivo)
    (bind _output_get (Variables|Default|SetPassoAttuale (+ (Variables|Default|GetPassoAttuale) 1)))
    (if (== _output_get 6)
      (Development|PrintString "ENIGMA RISOLTO"))
    (else
      (Variables|Default|SetPassoAttuale 0))))